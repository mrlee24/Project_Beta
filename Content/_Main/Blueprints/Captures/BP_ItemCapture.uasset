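; BP_ItemCapture is a scene capture actor that renders attached items for the inventory and equipment systems.
; On BeginPlay or InitializeCapture it caches the inventory and equipment components and passes itself to both.
; Start and End events toggle the SceneCaptureComponent2D's every-frame capture, limiting continuous rendering to when it is requested.
; Attach and detach events forward item data to AttachItem and DetachItem.
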(event `RPGCaptureInterface.StartCapture`
  ;[0 1 0.08226 0.227] Start Capture
  (set `SceneCaptureComponent.bCaptureEveryFrame` true (`self.SceneCaptureComponent2D`)))

(event `RPGCaptureInterface.EndCapture`
  ;[1 0 0.01016 0.269] End Capture
  (set `SceneCaptureComponent.bCaptureEveryFrame` false (`self.SceneCaptureComponent2D`)))

(event `RPGCaptureInterface.AttachToCapture`
  (params (ItemData :type "RPGItemData Structure"))
  ;[0.05725 1 0 0.248] Attach Item
  (`self.AttachItem` ItemData))

(event `RPGCaptureInterface.DetachFromCapture`
  (params (ItemData :type "RPGItemData Structure"))
  ;[1 0.02893 0 0.243] Detach Item
  (`self.DetachItem` ItemData))

(event `self.ReceiveBeginPlay`
  ;[0 0.3476 1 0.217] Set References
  (bind _returnvalue (`RPGInventoryFunctionLibrary.GetInventoryComponent` :!label _label))
  (bind _output_get (set `self.InventoryComponent` _returnvalue))
  (`RPGInventoryComponent.PassItemCaptureReference` _output_get self)
  (bind _returnvalue_2 (`RPGInventoryFunctionLibrary.GetEquipmentComponent`))
  (bind _output_get_2 (set `self.EquipmentComponent` _returnvalue_2))
  (`RPGEquipmentComponent.PassItemCaptureReference` _output_get_2 self))

(event `RPGCaptureInterface.InitializeCapture`
  ;[0 0.3476 1 0.217] Set References
  (goto _label))

(fn `UserConstructionScript`)