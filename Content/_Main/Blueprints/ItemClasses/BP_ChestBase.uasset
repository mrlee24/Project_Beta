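; BP_ChestBase is a base chest item that opens and closes in response to player interaction.
; OnInteraction plays a one-shot skeletal mesh animation and hides the interaction widget through ACInteractable.
; OnEndInteraction plays a one-shot animation, then shows the widget again after a short delay.
; The construction script only calls its parent.
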(event `RPGInteractableInterface.OnInteraction`
  ;[1 0 0.01444 0.2] Open / Close Chest
  (`SkeletalMeshComponent.PlayAnimation` (`self.SkeletalMesh`) null false)
  ;[0.1119 0 0.4072 0.2] Toggle Interaction Widget
  (`RPGInteractableComponent.ToggleInteractionWidget` (`self.AC_Interactable`) false))

(event `RPGInteractableInterface.OnEndInteraction`
  ;[1 0 0.01444 0.2] Open / Close Chest
  (`SkeletalMeshComponent.PlayAnimation` (`self.SkeletalMesh`) null false)
  ;[0.1119 0 0.4072 0.2] Toggle Interaction Widget
  (`KismetSystemLibrary.Delay` 0.2)
  (`RPGInteractableComponent.ToggleInteractionWidget` (`self.AC_Interactable`) true))

(fn `UserConstructionScript`
  (`parent.UserConstructionScript`))